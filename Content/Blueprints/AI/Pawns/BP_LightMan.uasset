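; BP_LightMan is an AI character with a spotlight and perception component that dies from point damage to its static mesh.
; Death sets Dead, hides mesh and light through MCDead, disables collision and movement, calls CallDeath and destroys perception.
; Capsule overlap with another LightMan launches that one toward this one's location at randomized speed.
; Unconnected debug logic prints perception's important locations and best target on authority.
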(event `self.ReceivePointDamage`
  (params (Damage :type "Float (single-precision)") (DamageType :type "DamageType Object Reference") (HitLocation :type "Vector Structure") (HitNormal :type "Vector Structure") (HitComponent :type "PrimitiveComponent Object Reference") (BoneName :type Name) (ShotFromDirection :type "Vector Structure") (InstigatedBy :type "Controller Object Reference") (DamageCauser :type "Actor Object Reference") (HitInfo :type "HitResult Structure (by ref)"))
  (if (== HitComponent (`self.StaticMesh`))
    (set `self.bDead` true)
    (`self.MC Dead`)
    (`PrimitiveComponent.SetCollisionEnabled` (`self.CapsuleComponent`) "NoCollision")
    (`CharacterMovementComponent.DisableMovement` (`self.CharacterMovement`))
    (`self.Death`)
    (`ActorComponent.K2_DestroyComponent` (`self.Perception`))))

(event `self.ReceiveTick`
  (params (DeltaSeconds :type "Float (single-precision)")))

(event `MC Dead`
  (`SceneComponent.SetHiddenInGame` (`self.StaticMesh`) true false)
  (`SceneComponent.SetHiddenInGame` (`self.SpotLight`) true false)
  (`PrimitiveComponent.SetCollisionEnabled` (`self.CapsuleComponent`) "NoCollision"))

(event `self.CapsuleComponent.OnComponentBeginOverlap`
  (params (OverlappedComponent :type "PrimitiveComponent Object Reference") (OtherActor :type "Actor Object Reference") (OtherComp :type "PrimitiveComponent Object Reference") (OtherBodyIndex :type Integer) (bFromSweep :type Boolean) (SweepResult :type "HitResult Structure (by ref)"))
  (bind _asbp_light_man (cast `/Game/Blueprints/AI/Pawns/BP_LightMan` OtherActor))
  (`self.LaunchCharacter` _asbp_light_man (* (`KismetMathLibrary.Normal` (- (`self.K2_GetActorLocation`) (`self.K2_GetActorLocation` _asbp_light_man))) (`KismetMathLibrary.RandomFloatInRange` 300.0 600.0)) true false))

(fn `UserConstructionScript`)