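; AI controller for BP_LightMan pawns that runs each pawn's own behavior tree.
; On BeginPlay, on the server only, it casts the controlled pawn, binds to its Death event and starts the behavior tree stored on that pawn.
; When the pawn dies, it stops the brain component, unpossesses and destroys itself.
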(event `self.ReceiveBeginPlay`
  (`/Engine/EditorBlueprintResources/ActorMacros.Switch Has Authority`
    (:`Authority`
      (bind _asbp_light_man (cast `/Game/Blueprints/AI/Pawns/BP_LightMan` (`self.K2_GetPawn`)))
      (add `/Game/Blueprints/AI/Pawns/BP_LightMan.Death` _asbp_light_man (delegate `PosessedDead`))
      (`self.RunBehaviorTree` (`/Game/Blueprints/AI/Pawns/BP_LightMan.Behavior` _asbp_light_man)))))

(event `PosessedDead`
  (`BrainComponent.StopLogic` (`self.BrainComponent`) "Dead")
  (`self.UnPossess`)
  (`self.K2_DestroyActor`))

(fn `UserConstructionScript`)