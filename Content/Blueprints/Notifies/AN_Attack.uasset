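; AN_Attack is an animation notify that lands an attack hit when the montage or animation reaches it.
; It sphere-traces on Visibility at a named mesh socket, ignoring the owner, and adds unique hit actors to DamagedActors, which is never cleared here.
; Every listed actor takes fixed damage credited to the owner, and Characters are also launched away from the owner and upward.
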(fn `Received_Notify`
  (params (MeshComp :type "SkeletalMeshComponent Object Reference") (Animation :type "AnimSequenceBase Object Reference") (EventReference :type "AnimNotifyEventReference Structure (by ref)"))
  (returns (ReturnValue :type Boolean))
  (locals (DamagedActors :type "Array of Actor Object Reference"))
  (bind _returnvalue (`SceneComponent.GetSocketLocation` MeshComp (`self.In Socket Name`)))
  (bind _returnvalue_2 (`ActorComponent.GetOwner` (`local.MeshComp`)))
  (bind _outhits (`KismetSystemLibrary.SphereTraceMulti` _returnvalue (+ _returnvalue (0.0 0.0 1.0)) 150.0 "TraceTypeQuery1" false (`|MakeArray` (`ActorComponent.GetOwner` MeshComp))))
  (for _array_element _outhits
    (`KismetArrayLibrary.Array_AddUnique` (`local.DamagedActors`) (`.HitActor` (`GameplayStatics.BreakHitResult` _array_element))))
  (for _array_element_2 (`local.DamagedActors`)
    (`GameplayStatics.ApplyDamage` _array_element_2 33.333333 null _returnvalue_2)
    (bind _ascharacter (cast `Character` _array_element_2))
    (`Character.LaunchCharacter` _ascharacter (+ (* (`KismetMathLibrary.Normal` (- (`Actor.K2_GetActorLocation` _ascharacter) (`Actor.K2_GetActorLocation` _returnvalue_2))) 500.0) (0.0 0.0 500.0)) false false))
  (return true))