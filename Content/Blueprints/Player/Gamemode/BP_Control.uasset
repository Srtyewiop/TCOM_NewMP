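; BP_Control is the player controller that handles role selection and spawning for Police, Medic, Mystic and Lumber characters.
; The local controller shows the selection widget on BeginPlay.
; SRSpawn spawns and possesses the chosen role at its tagged spawn point and updates the game mode, or reopens selection if that role already exists.
; On unpossess, the authority spawns and possesses a BP_POVspec pawn at the old pawn's transform.
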(event `self.ReceiveUnPossess`
  (params (UnpossessedPawn :type "Pawn Object Reference"))
  (`/Engine/EditorBlueprintResources/ActorMacros.Switch Has Authority`
    (:`Authority`
      (bind _returnvalue (`|SpawnActorFromClass` "/Game/Blueprints/Player/Gamemode/BP_POVspec.BP_POVspec_C" (`self.GetTransform` UnpossessedPawn) "AlwaysSpawn" "MultiplyWithRoot" null null))
      (`self.Possess` _returnvalue))))

(event `SR Spawn`
  (params (Type :type Integer))
  (bind _returnvalue (select `int` Type :`0` "/Game/Blueprints/Player/BP_Police.BP_Police_C" :`1` "/Game/Blueprints/Player/BP_Medic.BP_Medic_C" :`2` "/Game/Blueprints/Player/BP_Mystic.BP_Mystic_C" :`3` "/Game/Blueprints/Player/BP_Lumber.BP_Lumber_C" :!type "Actor Class Reference"))
  (bind _outactors (`GameplayStatics.GetAllActorsOfClass` _returnvalue))
  (if (== (`KismetArrayLibrary.Array_Length` _outactors) 0)
    (bind _outactors_2 (`GameplayStatics.GetAllActorsWithTag` (select `int` Type :`0` "Spawn_Police" :`1` "Spawn_Medic" :`2` "Spawn_Mystic" :`3` "Spawn_Lumber" :!type "Name")))
    (bind _returnvalue_2 (`|SpawnActorFromClass` _returnvalue (`self.GetTransform` (`|GetArrayItem` _outactors_2)) "AlwaysSpawn" "MultiplyWithRoot" null null))
    (bind _asbp_player (cast `/Game/Blueprints/Player/BP_Player` _returnvalue_2))
    (`self.Possess` _asbp_player)
    (bind _asthird_person_game_mode (cast `/Game/Blueprints/Player/Gamemode/ThirdPersonGameMode` (`GameplayStatics.GetGameMode`)))
    (`/Game/Blueprints/Player/Gamemode/ThirdPersonGameMode.UpdatePlayers` _asthird_person_game_mode Type)
    (else
      (`self.CL Select`))))

(event `CL Select`
  (bind _returnvalue (`|CreateWidget` "/Game/Blueprints/Player/WB_SelectPlayer.WB_SelectPlayer_C" self))
  (`UserWidget.AddToPlayerScreen` _returnvalue 0))

(event `self.ReceiveBeginPlay`
  (if (`self.IsLocalController`)
    (bind _returnvalue (`|CreateWidget` "/Game/Blueprints/Player/WB_SelectPlayer.WB_SelectPlayer_C" self))
    (`UserWidget.AddToPlayerScreen` _returnvalue 0)))

(fn `UserConstructionScript`)