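; BP_POVspec is a spectator that shows living BP_Player characters from first-person view, cycling between them with UseAbility.
; It rebuilds the living-player list every Tick and interpolates its transform toward the watched player's LampScene.
; A velocity-scaled cosine adds camera bob.
; Switching restores the previous target, then exposes the new one's owner-only pistol and lamp while hiding its mesh, LampAll and Ability.
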(event `self.ReceiveTick`
  (params (DeltaSeconds :type "Float (single-precision)"))
  (bind _camera (`self.Camera`))
  (bind (_relativelocation_x _relativelocation_y _relativelocation_z) (`KismetMathLibrary.BreakVector` (`SceneComponent.RelativeLocation` _camera)))
  (`|ExecutionSequence`
    (:`then_0`
      (`KismetArrayLibrary.Array_Clear` (`self.Players`))
      (bind _outactors (`GameplayStatics.GetAllActorsOfClass` "/Game/Blueprints/Player/BP_Player.BP_Player_C"))
      (for _array_element _outactors
        (if (not (`/Game/Blueprints/Player/BP_Player.bDead` _array_element))
          (`KismetArrayLibrary.Array_AddUnique` (`self.Players`) _array_element))))
    (:`then_1`
      (bind _current (`self.Current`)
        (:`then`
          (`self.K2_SetActorTransform` (`KismetMathLibrary.TInterpTo` (`self.GetTransform`) (`SceneComponent.K2_GetComponentToWorld` (`/Game/Blueprints/Player/BP_Player.LampScene` _current)) (`GameplayStatics.GetWorldDeltaSeconds`) 30.0))
          (`SceneComponent.K2_SetRelativeLocation` _camera (`KismetMathLibrary.MakeVector` 0.0 0.0 (`KismetMathLibrary.FInterpTo` _relativelocation_z (* (`KismetMathLibrary.Cos` (* (`KismetSystemLibrary.GetGameTimeInSeconds`) 12.0)) (/ (`KismetMathLibrary.VSize` (`self.GetVelocity` _current)) 300.0) 25.0) (`GameplayStatics.GetWorldDeltaSeconds`) 5.0)) false false))
        (:`else`)))))

(event `self.ReceiveBeginPlay`
  (bind _outactors (`GameplayStatics.GetAllActorsOfClass` "/Game/Blueprints/Player/BP_Player.BP_Player_C"))
  (for _array_element _outactors
    (if (not (`/Game/Blueprints/Player/BP_Player.bDead` _array_element))
      (`KismetArrayLibrary.Array_AddUnique` (`self.Players`) _array_element)))
  (`KismetSystemLibrary.Delay` 0.2)
  (if (`self.IsLocallyControlled`)
    (`self.update`)))

(event `InputAction|UseAbility`
  (params (Key :type "Key Structure"))
  (:`Pressed`
    (`self.update`)))

(event `update`
  (`self.PosessLocal` false (`self.Current`))
  (`self.PosessLocal` true (`|GetArrayItem` (`self.Players`) (`self.index`)))
  (`self.SR Attach`))

(event `SR Attach`
  (set `self.Current` (`|GetArrayItem` (`self.Players`) (`self.index`)))
  (bind _result (`/Engine/EditorBlueprintResources/StandardMacros.IncrementInt` (`self.index`))
    (:`  `
      (if (> _result (`KismetArrayLibrary.Array_LastIndex` (`self.Players`)))
        (set `self.index` 0)))))

(event `PosessLocal`
  (params (Start :type Boolean) (InputPin :type "/Game/Blueprints/Player/BP_Player Object Reference"))
  (`/Engine/EditorBlueprintResources/StandardMacros.IsValid` InputPin
    (:`Is Valid`
      (`PrimitiveComponent.SetOnlyOwnerSee` (`/Game/Blueprints/Player/BP_Player.PistolSelf` InputPin) (not Start))
      (`PrimitiveComponent.SetOnlyOwnerSee` (`/Game/Blueprints/Player/BP_Player.LampSelf` InputPin) (not Start))
      (`SceneComponent.SetHiddenInGame` (`Character.Mesh` InputPin) Start false)
      (`SceneComponent.SetHiddenInGame` (`/Game/Blueprints/Player/BP_Player.LampAll` InputPin) Start false)
      (`SceneComponent.SetHiddenInGame` (`/Game/Blueprints/Player/BP_Player.Ability` InputPin) Start false))))

(fn `UserConstructionScript`)