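; BP_Medic is the medic player class, with an ability that heals another player or the medic.
; AbilityEffect runs a short sphere trace from the camera along the control rotation, heals a hit BP_Player below full HP and spends a use, then always clears Prepared.
; AltAbility self-heals when prepared, hurt and holding uses, then spends a use and clears Prepared.
; The trace still has timed debug drawing enabled.
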(event `self.AbilityEffect`
  (bind _returnvalue (`SceneComponent.K2_GetComponentLocation` (`self.CamS`)))
  (`|ExecutionSequence`
    (:`then_0`
      (bind _outhit (`KismetSystemLibrary.SphereTraceSingle` :`Start` _returnvalue :`End` (+ _returnvalue (* (`KismetMathLibrary.GetForwardVector` (`self.GetControlRotation`)) 50.0)) :`Radius` 25.0 :`TraceChannel` "TraceTypeQuery1" :`DrawDebugType` "ForDuration"))
      (bind _asbp_player (cast `/Game/Blueprints/Player/BP_Player` (`.HitActor` (`GameplayStatics.BreakHitResult` _outhit))))
      (if (< (`/Game/Blueprints/Player/BP_Player.HP` _asbp_player) 100.0)
        (`self.Heal` _asbp_player 50.0)
        (`/Engine/EditorBlueprintResources/StandardMacros.DecrementInt` (`self.AbilityUses`))))
    (:`then_1`
      (set `self.bPrepared` false))))

(event `self.AltAbility`
  (if (and (> (`self.AbilityUses`) 0) (< (`self.HP`) 100.0) (`self.bPrepared`))
    (`self.Heal` 50.0)
    (set `self.bPrepared` false)
    (`/Engine/EditorBlueprintResources/StandardMacros.DecrementInt` (`self.AbilityUses`))))

(fn `UserConstructionScript`
  (`parent.UserConstructionScript`))