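; BP_Lumber is a child player Blueprint whose ability is a short-range melee strike.
; AbilityEffect sphere-traces from the camera along control rotation and damages the hit actor, guarded against re-triggering by UsingAbilty.
; The AttackAnim timeline swings PistolScene's pitch, then a short delay clears the Prepared and in-use flags.
; PepareAbilityVisuals interpolates PistolScene between readied and idle rotations based on Prepared.
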(event `self.AbilityEffect`
  (bind _pistolscene (`self.PistolScene`))
  (bind _returnvalue (`SceneComponent.K2_GetComponentLocation` (`self.CamS`)))
  (bind (_relativerotation_roll _relativerotation_pitch _relativerotation_yaw) (`KismetMathLibrary.BreakRotator` (`SceneComponent.RelativeRotation` _pistolscene)))
  (if (not (`self.UsingAbilty`))
    (set `self.UsingAbilty` true)
    (bind _outhit (`KismetSystemLibrary.SphereTraceSingle` :`Start` _returnvalue :`End` (+ _returnvalue (* (`KismetMathLibrary.GetForwardVector` (`self.GetControlRotation`)) 70.0)) :`Radius` 25.0 :`TraceChannel` "TraceTypeQuery1" :`DrawDebugType` "ForDuration"))
    (`GameplayStatics.ApplyDamage` (`.HitActor` (`GameplayStatics.BreakHitResult` _outhit)) 25.0 null self)
    (bind (_direction _newtrack_0) (`Timeline|AttackAnim` :!via `PlayFromStart`)
      (:`Update`
        (`SceneComponent.K2_SetRelativeRotation` _pistolscene (`KismetMathLibrary.MakeRotator` _relativerotation_roll _newtrack_0 _relativerotation_yaw) false false))
      (:`Finished`
        (`KismetSystemLibrary.Delay` 0.5)
        (set `self.bPrepared` false)
        (set `self.UsingAbilty` false)))))

(fn `PepareAbilityVisuals`
  (bind _pistolscene (`self.PistolScene`))
  (`SceneComponent.K2_SetRelativeRotation` _pistolscene (`KismetMathLibrary.RInterpTo` (`SceneComponent.RelativeRotation` _pistolscene) (select `bool` (`self.bPrepared`) :`false` (struct :`Pitch` -60.0 :`Yaw` 90.0 :`Roll` -90.0) :`true` (struct :`Pitch` -15.0 :`Yaw` 35.0) :!type "Rotator Structure") (`GameplayStatics.GetWorldDeltaSeconds`) 15.0) false false))

(fn `UserConstructionScript`
  (`parent.UserConstructionScript`))